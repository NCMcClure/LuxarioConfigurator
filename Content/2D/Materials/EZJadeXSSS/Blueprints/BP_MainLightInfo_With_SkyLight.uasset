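; Actor that feeds main directional light and sky light data into the MP_SphereProbeSSS material parameter collection, apparently for the jade subsurface scattering materials.
; SetLight runs on construction and every Tick to keep the collection in sync with the lights.
; It writes the negated light forward vector as Light Direction and color times intensity as Light Color.
; Ambient sums the directional light's indirect contribution, sky light and an adjustable environment color.
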(event EventBeginPlay)

(event Collision|EventActorBeginOverlap
  (params (OtherActor :type Actor%20Object%20Reference)))

(event EventTick
  (params (DeltaSeconds :type Float%20%28single-precision%29))
  (CallFunction|SetLight))

(fn ConstructionScript
  (CallFunction|SetLight))

(fn SetLight
  (bind _directional_light_actor (Variables|Default|GetDirectional%20Light%20Actor))
  (bind _sky_light_actor (Variables|Default|GetSky%20Light%20Actor))
  (bind _returnvalue (Actor|GetComponentbyClass _sky_light_actor "/Script/Engine.SkyLightComponent"))
  (bind _lightcomponent (Variables|/Script/Engine.Light|GetLightComponent _directional_light_actor))
  (bind _returnvalue_2 (Rendering|Components|Light|GetLightColor _lightcomponent))
  (Rendering|Material|SetVectorParameterValue "/Game/2D/Materials/EZJadeXSSS/Materials/MP_SphereProbeSSS.MP_SphereProbeSSS" "Light Direction" (Math|Conversions|ToLinearColor(Vector) (Math|Vector|NegateVector (Math|Rotator|GetRotationXVector (Transformation|GetActorRotation _directional_light_actor)))) :!class /Script/Engine.KismetMaterialLibrary)
  (Rendering|Material|SetVectorParameterValue "/Game/2D/Materials/EZJadeXSSS/Materials/MP_SphereProbeSSS.MP_SphereProbeSSS" "Light Color" (* _returnvalue_2 (Variables|/Script/Engine.LightComponentBase|GetIntensity _lightcomponent)) :!class /Script/Engine.KismetMaterialLibrary)
  (Rendering|Material|SetVectorParameterValue "/Game/2D/Materials/EZJadeXSSS/Materials/MP_SphereProbeSSS.MP_SphereProbeSSS" "Ambient" (Math|Conversions|ToLinearColor(Vector) (+ (+ (Math|Conversions|ToVector(LinearColor) (* _returnvalue_2 (Variables|/Script/Engine.LightComponentBase|GetIndirectLightingIntensity _lightcomponent))) (Math|Conversions|ToVector(LinearColor) (* (Rendering|Components|Light|GetLightColor _returnvalue) (Variables|/Script/Engine.LightComponentBase|GetIntensity _returnvalue)))) (* (Variables|Default|GetEnvironment%20Color) (Variables|Default|GetEnviroment%20Intensity)))) :!class /Script/Engine.KismetMaterialLibrary))