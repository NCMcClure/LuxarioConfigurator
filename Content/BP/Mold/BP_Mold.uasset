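; BP_Mold is a two-part mold whose shape is set by arch, concave depth and width, dips and kicks parameters.
; UpdateMorphs writes these values to morph targets on top and bottom skeletal meshes, each split into main, sides and walls components.
; Each component receives only the parameters relevant to it, with matching values on both halves.
; The construction script calls UpdateMorphs, and no Tick or BeginPlay logic runs.
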(event Custom|UpdateMorphs
  (Utilities|FlowControl|Sequence
    (:then_0
      (Components|SkeletalMesh|SetMorphTarget (Variables|Default|GetSKSH_Mold_Bottom) "Concave_Width_Bottom" (Variables|Default|GetConcaveWidth) true)
      (Components|SkeletalMesh|SetMorphTarget (Variables|Default|GetSKSH_Mold_Bottom) "Kicks_Bottom" (Variables|Default|GetKicks) true)
      (Components|SkeletalMesh|SetMorphTarget (Variables|Default|GetSKSH_Mold_Top) "Concave_Width_Top" (Variables|Default|GetConcaveWidth) true)
      (Components|SkeletalMesh|SetMorphTarget (Variables|Default|GetSKSH_Mold_Top) "Kicks_Top" (Variables|Default|GetKicks) true))
    (:then_1
      (Components|SkeletalMesh|SetMorphTarget (Variables|Default|GetSKSH_Mold_Bottom_Sides) "Arch_Bottom_Sides" (Variables|Default|GetArch) true)
      (Components|SkeletalMesh|SetMorphTarget (Variables|Default|GetSKSH_Mold_Bottom_Sides) "Concave_Depth_Bottom_Sides" (Variables|Default|GetConcaveDepth) true)
      (Components|SkeletalMesh|SetMorphTarget (Variables|Default|GetSKSH_Mold_Bottom_Sides) "Dips_Bottom_Sides" (Variables|Default|GetDips) true)
      (Components|SkeletalMesh|SetMorphTarget (Variables|Default|GetSKSH_Mold_Bottom_Sides) "Kicks_Bottom_Sides" (Variables|Default|GetKicks) true)
      (Components|SkeletalMesh|SetMorphTarget (Variables|Default|GetSKSH_Mold_Top_Sides) "Arch_Top_Sides" (Variables|Default|GetArch) true)
      (Components|SkeletalMesh|SetMorphTarget (Variables|Default|GetSKSH_Mold_Top_Sides) "Concave_Depth_Top_Sides" (Variables|Default|GetConcaveDepth) true)
      (Components|SkeletalMesh|SetMorphTarget (Variables|Default|GetSKSH_Mold_Top_Sides) "Dips_Top_Sides" (Variables|Default|GetDips) true)
      (Components|SkeletalMesh|SetMorphTarget (Variables|Default|GetSKSH_Mold_Top_Sides) "Kicks_Top_Sides" (Variables|Default|GetKicks) true))
    (:then_2
      (Components|SkeletalMesh|SetMorphTarget (Variables|Default|GetSKSH_Mold_Bottom_Walls) "Arch_Bottom_Walls" (Variables|Default|GetArch) true)
      (Components|SkeletalMesh|SetMorphTarget (Variables|Default|GetSKSH_Mold_Bottom_Walls) "Concave_Depth_Bottom_Walls" (Variables|Default|GetConcaveDepth) true)
      (Components|SkeletalMesh|SetMorphTarget (Variables|Default|GetSKSH_Mold_Bottom_Walls) "Dips_Bottom_Walls" (Variables|Default|GetDips) true)
      (Components|SkeletalMesh|SetMorphTarget (Variables|Default|GetSKSH_Mold_Bottom_Walls) "Concave_Width_Bottom_Walls" (Variables|Default|GetConcaveWidth) true)
      (Components|SkeletalMesh|SetMorphTarget (Variables|Default|GetSKSH_Mold_Top_Walls) "Arch_Top_Walls" (Variables|Default|GetArch) true)
      (Components|SkeletalMesh|SetMorphTarget (Variables|Default|GetSKSH_Mold_Top_Walls) "Concave_Depth_Top_Walls" (Variables|Default|GetConcaveDepth) true)
      (Components|SkeletalMesh|SetMorphTarget (Variables|Default|GetSKSH_Mold_Top_Walls) "Dips_Top_Walls" (Variables|Default|GetDips) true)
      (Components|SkeletalMesh|SetMorphTarget (Variables|Default|GetSKSH_Mold_Top_Walls) "Concave_Width_Top_Walls" (Variables|Default|GetConcaveWidth) true))))

(event EventBeginPlay)

(event Collision|EventActorBeginOverlap
  (params (OtherActor :type Actor%20Object%20Reference)))

(event EventTick
  (params (DeltaSeconds :type Float%20%28single-precision%29)))

(fn ConstructionScript
  (CallFunction|UpdateMorphs))